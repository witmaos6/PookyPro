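; BP_Runner is a runner Blueprint whose Turning event smoothly rotates it by a given yaw angle.
; The event stores the current yaw and the target, then plays the TurnRight timeline from the start to interpolate between them.
; Each timeline update sets the relative rotation, then rounds the resulting actor yaw to a whole degree.
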(event EventTurning
  (params (Angle :type Float%20%28single-precision%29))
  (bind _output_get (Variables|Default|SetCurrentAngle (.yaw (Transformation|GetActorRotation))))
  (bind _output_get_2 (Variables|Default|SetAngleRotation (+ _output_get Angle)))
  (bind _angle (Timeline|TurnRight PlayFromStart)
    (:Update
      (Transformation|SetActorRelativeRotation (Math|Rotator|MakeRotator 0.0 0.0 (Math|Float|Lerp (Variables|Default|GetCurrentAngle) _output_get_2 _angle)))
      (Transformation|SetActorRotation (Math|Rotator|MakeRotator 0.0 0.0 (Math|Conversions|ToFloat(Integer) (Math|Float|Round (.yaw (Transformation|GetActorRotation)))))))))

(fn ConstructionScript)