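; BP_RailChange is a trigger actor that shifts the runner from rail 0 to rail 1 when it overlaps the box.
; On overlap it sets the player controller's LeftRail to 1 and, if CurrentRail is 0, starts a timeline.
; The timeline lerps the runner diagonally from its captured location, using its forward and right vectors.
; On finish it re-enables rail changing and updates CurrentRail.
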(event OnComponentBeginOverlap(Box)
  (params (OverlappedComponent :type Primitive%20Component%20Object%20Reference) (OtherActor :type Actor%20Object%20Reference) (OtherComp :type Primitive%20Component%20Object%20Reference) (OtherBodyIndex :type Integer) (bFromSweep :type Boolean) (SweepResult :type Hit%20Result%20Structure%20%28by%20ref%29))
  (bind _asbp_runner (Utilities|Casting|CastToBP_Runner OtherActor))
  (bind _asbp_runner_player_controller (Utilities|Casting|CastToBP_RunnerPlayerController (Pawn|GetController _asbp_runner))
    (:then
      (Variables|/Script/First.RunnerPlayerController|SetLeftRail _asbp_runner_player_controller 1)
      (Variables|Default|SetNewVar (Transformation|GetActorLocation _asbp_runner))
      (if (== (Variables|/Script/First.RunnerPlayerController|GetCurrentRail _asbp_runner_player_controller) 0)
        (bind _changetime (Timeline|타임라인 PlayFromStart)
          (:Update
            (Transformation|SetActorLocation _asbp_runner (Math|Vector|Lerp(Vector) (Variables|Default|GetNewVar) (+ (Variables|Default|GetNewVar) (+ (* (Math|Vector|GetForwardVector (Transformation|GetActorRotation _asbp_runner)) (Math|Conversions|ToVector(Float) (Variables|/Script/First.Runner|GetDiagonalTravelDistance _asbp_runner))) (* (Math|Vector|GetRightVector (Transformation|GetActorRotation _asbp_runner)) (* (Variables|/Script/First.RunnerPlayerController|GetMoveInterval _asbp_runner_player_controller) 1.0)))) _changetime) false false))
          (:Finished
            (Variables|/Script/First.RunnerPlayerController|SetbRailsChangeable _asbp_runner_player_controller true)
            (Variables|/Script/First.RunnerPlayerController|SetCurrentRail _asbp_runner_player_controller 1 :!label _label)))))
    (:CastFailed
      (goto _label))))

(event EventBeginPlay)

(event Collision|EventActorBeginOverlap
  (params (OtherActor :type Actor%20Object%20Reference)))

(event EventTick
  (params (DeltaSeconds :type Float%20%28single-precision%29)))

(fn ConstructionScript)